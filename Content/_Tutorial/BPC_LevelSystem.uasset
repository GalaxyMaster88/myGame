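; Level system component that tracks the player's XP, level and points and shows them on the HUD.
; On begin play it restores saved progress from the game instance and pushes level and points to the HUD after a short delay.
; XP gains are saved and can trigger recursive level-ups, each raising the XP threshold by half, granting a point and adding any milestone bonus from a level-keyed map.
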(event Custom|Update%20XP
  (params (Add%20XP :type Integer))
  (bind _output_get (Variables|Default|SetCurrentXP (+ Add%20XP (Variables|Default|GetCurrentXP))))
  (Development|PrintString (Utilities|String|ToString(Integer) _output_get))
  (Default|AddEXPNumber (Variables|Default|GetBP_HUD_Base) Add%20XP)
  (Class|BPISave|SavePlayerLevel(Message) (Game|GetGameInstance) (Utilities|Struct|MakeS_PlayerLevelSave (Variables|Default|GetCurrentXP) (Variables|Default|GetMaxXP) (Variables|Default|GetLevel) (Variables|Default|GetPoints)))
  (if (>= (Variables|Default|GetCurrentXP) (Variables|Default|GetMaxXP))
    (CallFunction|LevelUp)))

(event Custom|Level%20Up
  (Variables|Default|SetCurrentXP (- (Variables|Default|GetCurrentXP) (Variables|Default|GetMaxXP)))
  (Variables|Default|SetMaxXP (+ (/ (Variables|Default|GetMaxXP) 2) (Variables|Default|GetMaxXP)))
  (bind _result (Math|Integer|IncrementInt (Variables|Default|GetLevel))
    (:%20%20
      (Default|ShowLevelUp (Variables|Default|GetBP_HUD_Base) _result)
      (CallFunction|CheckLevelMilestoneReward)
      (bind _result_2 (Math|Integer|IncrementInt (Variables|Default|GetPoints))
        (:%20%20
          (Variables|/Script/UMG.TextBlock|SetText (Variables|/Game/FirstPerson/Blueprints/PlayerHUD.PlayerHUD_C|GetPoints (Variables|Default|Getplayer%20HUD)) (Utilities|Text|ToText(String) (Utilities|String|BuildString(Integer) "" "POINTS: " _result_2)))
          (Class|BPISave|SavePlayerLevel(Message) (Game|GetGameInstance) (Utilities|Struct|MakeS_PlayerLevelSave (Variables|Default|GetCurrentXP) (Variables|Default|GetMaxXP) (Variables|Default|GetLevel) (Variables|Default|GetPoints)))
          (if (>= (Variables|Default|GetCurrentXP) (Variables|Default|GetMaxXP))
            (CallFunction|LevelUp)))))))

(event EventBeginPlay
  (Utilities|FlowControl|Sequence
    (:then_0
      (bind _savegamedata (Class|BPISave|GetGameData(Message) (Game|GetGameInstance)))
      (Utilities|IsValid _savegamedata
        (:Is%20Valid
          (CallFunction|LoadPlayerLevel (Variables|/Game/_Tutorial/BP_SaveGame.BP_SaveGame_C|GetS_PlayerLevelSave _savegamedata)))))
    (:then_1
      (Utilities|FlowControl|Delay 0.1)
      (bind _asplayer_hudclass (Utilities|Casting|CastToPlayerHUDClass (HUD|GetHUD (Game|GetPlayerController 0))))
      (bind _output_get (Variables|Default|SetBP_HUD_Base _asplayer_hudclass))
      (Default|AddLeveltoHUD _output_get (Variables|Default|GetLevel))
      (Variables|Default|Setplayer%20HUD (Variables|/Game/FirstPerson/Blueprints/PlayerHUDClass.PlayerHUDClass_C|GetMain%20HUD _output_get))
      (Default|AddPointstoHUD _output_get (Variables|Default|GetPoints)))))

(fn CheckLevelMilestoneReward
  (bind _keys (Utilities|Map|Keys (Variables|Default|GetLevelMilestoneReward)))
  (for _array_element _keys
    (if (== _array_element (Variables|Default|GetLevel))
      (Variables|Default|SetPoints (+ (Variables|Default|GetPoints) (.Value (Utilities|Map|Find (Variables|Default|GetLevelMilestoneReward) _array_element)))))))

(fn LoadPlayerLevel
  (params (PlayerLevelSave :type S%20Player%20Level%20Save%20Structure))
  (Utilities|FlowControl|Sequence
    (:then_0
      (Variables|Default|SetCurrentXP (.currentxp PlayerLevelSave)))
    (:then_1
      (if (!= (.maxxp PlayerLevelSave) 0)
        (Variables|Default|SetMaxXP (.maxxp PlayerLevelSave))))
    (:then_2
      (if (!= (.level PlayerLevelSave) 0)
        (Variables|Default|SetLevel (.level PlayerLevelSave))))
    (:then_3
      (Variables|Default|SetPoints (.points PlayerLevelSave)))))